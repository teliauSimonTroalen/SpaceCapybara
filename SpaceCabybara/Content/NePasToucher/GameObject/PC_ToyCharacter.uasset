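; PC_ToyCharacter is a player character Blueprint with wall-running and landing handling for a smash move.
; WallRunActivation traces left and right while falling, aligns the character to the hit wall, sets horizontal velocity and removes gravity until OffWall restores it.
; Landing resets control roll and gravity, clears the smash flag and updates the interface widget.
; Tick, CameraTilt and IsMovingForward are empty, and BoostOffWall is only called from unreachable nodes.
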(event Custom|WallRunActivation
  (bind _returnvalue (Transformation|GetActorForwardVector))
  (bind _returnvalue_2 (Transformation|GetActorForwardVector))
  (bind _returnvalue_3 (Transformation|GetActorLocation))
  (bind _returnvalue_4 (Transformation|GetActorLocation))
  (bind _velocityonwall (Variables|Default|GetVelocityOnWall))
  (bind _charactermovement (Variables|Character|GetCharacterMovement))
  (bind _velocityonwall_2 (Variables|Default|GetVelocityOnWall))
  (bind _charactermovement_2 (Variables|Character|GetCharacterMovement))
  (bind _returnvalue_5 (* _returnvalue _velocityonwall_2))
  (bind _returnvalue_6 (* _returnvalue_2 _velocityonwall))
  ;[1 1 1] wall detection
  (if (AI|Components|NavMovement|IsFalling (Variables|Character|GetCharacterMovement))
    ;;[1 1 1] check wall side
    (Utilities|FlowControl|Sequence
      (:then_0
        ;;[0.3252 0.1789 0.8177] Run on the right side of the wall
        (bind (_outhit _returnvalue_7) (Collision|LineTraceByChannel _returnvalue_4 (+ _returnvalue_4 (* (Transformation|GetActorRightVector) 50)) "TraceTypeQuery1" false 0 "ForDuration"))
        (if _returnvalue_7
          (Variables|Default|SetIsRightSide true)
          (Variables|Default|SetOnRightSide true)
          (if (not (Variables|Default|GetIsJumpingOffWall))
            (Transformation|SetActorRotation (Math|Rotator|MakeRotator 0.0 0.0 (+ (.yaw (Math|Conversions|RotationFromXVector (.Normal (Collision|BreakHitResult _outhit)))) 9e+01)))
            (Variables|/Script/Engine.MovementComponent|SetVelocity _charactermovement (Math|Vector|MakeVector (.x _returnvalue_5) (.y _returnvalue_5) 0.0))
            (Variables|/Script/Engine.CharacterMovementComponent|SetGravityScale _charactermovement 0.0)
            (Class|MovementComponent|SetPlaneConstraintNormal _charactermovement "0, 0, 0")
            (CallFunction|CameraTilt 0.0))
          (else
            (Variables|Default|SetIsRightSide false)
            (CallFunction|OffWall))))
      (:then_1
        ;;[0.2205 0.6823 0.1634] Run on the Left side of the wall
        (bind (_outhit_2 _returnvalue_8) (Collision|LineTraceByChannel _returnvalue_3 (+ _returnvalue_3 (* (Transformation|GetActorRightVector) -50)) "TraceTypeQuery1" false 0 "ForDuration"))
        (if _returnvalue_8
          (Variables|Default|SetIsLeftSide true)
          (Variables|Default|SetOnRightSide false)
          (if (not (Variables|Default|GetIsJumpingOffWall))
            (Transformation|SetActorRotation (Math|Rotator|MakeRotator 0.0 0.0 (+ (.yaw (Math|Conversions|RotationFromXVector (.Normal (Collision|BreakHitResult _outhit_2)))) -9e+01)))
            (Variables|/Script/Engine.MovementComponent|SetVelocity _charactermovement_2 (Math|Vector|MakeVector (.x _returnvalue_6) (.y _returnvalue_6) 0.0))
            (Variables|/Script/Engine.CharacterMovementComponent|SetGravityScale _charactermovement_2 0.0)
            (Class|MovementComponent|SetPlaneConstraintNormal _charactermovement_2 "0, 0, 0")
            (CallFunction|CameraTilt 0.0))
          (else
            (Variables|Default|SetIsLeftSide false)
            (CallFunction|OffWall)))))))

(event Custom|LandedDelegate_Event
  (params (Hit :type Hit%20Result%20Structure%20%28by%20ref%29))
  (bind _returnvalue (Pawn|GetController))
  (bind _returnvalue_2 (Pawn|GetDesiredRotation _returnvalue))
  (Pawn|SetControlRotation _returnvalue (Math|Rotator|MakeRotator 0.0 (.pitch _returnvalue_2) (.yaw _returnvalue_2)))
  (Variables|/Script/Engine.CharacterMovementComponent|SetGravityScale (Variables|Character|GetCharacterMovement) 1.25)
  (Variables|Default|SetIsHulkSmashing false)
  (Default|DisplaySmash (Variables|Default|GetWidgetInterface)))

(event Custom|OffWall
  ;[1 1 1] When Off wall set gravity back to normal
  (Variables|/Script/Engine.CharacterMovementComponent|SetGravityScale (Variables|Character|GetCharacterMovement) 1.0))

(event Custom|WallRun
  ;[1 1 1] wall detection
)

(event EventBeginPlay
  (EventDispatchers|BindEventtoLandedDelegate (delegate Custom|LandedDelegate_Event))
  (Class|MovementComponent|SetPlaneConstraintEnabled (Variables|Character|GetCharacterMovement) true)
  (bind _foundwidgets (Widget|GetAllWidgetsOfClass "/Game/Teliau/Blueprint/UI/WI_Interface.WI_Interface_C" true))
  (Variables|Default|SetWidgetInterface (Utilities|Array|Get(acopy) _foundwidgets)))

(event EventTick
  (params (DeltaSeconds :type Float%20%28single-precision%29))
  ;[1 1 1] wall detection
)

(fn ConstructionScript)

(fn CameraTilt
  (params (Target%20X%28roll%29 :type Float%20%28double-precision%29)))

(fn BoostOffWall
  (bind _returnvalue (Transformation|GetActorRightVector))
  (bind _boostdir (Variables|Default|GetBoostDir))
  (Character|LaunchCharacter (Math|Vector|MakeVector (* (.x _returnvalue) _boostdir) (* (.y _returnvalue) _boostdir) 0.0) false false))