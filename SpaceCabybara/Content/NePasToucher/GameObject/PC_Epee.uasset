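; Thrown sword projectile that lets the player teleport onto and take possession of enemies.
; BeginPlay launches it by physics force away from the player; after a delay it interpolates back and is destroyed, unless stuck in an "Interupteur" switch.
; Hitting an "Ennemi" calls possession and runs a timeline gliding the player and camera to that enemy.
; The timeline then destroys enemy and sword, redirecting the player's prior velocity along the enemy's facing, portal-style.
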(event Custom|OnActorHit_Event
  (params (SelfActor :type Actor%20Object%20Reference) (OtherActor :type Actor%20Object%20Reference) (NormalImpulse :type Vector) (Hit :type Hit%20Result%20Structure%20%28by%20ref%29))
  (bind _pc_toy (Variables|Default|GetPC%20Toy))
  (bind _cube (Variables|Default|GetCube))
  ;[1 1 1] Tp du joueur sur l'ennemi
  ;;[0.4417 0.5036 1] TP Joueur
  (if (Actor|ActorHasTag OtherActor "Ennemi")
    (Variables|/Script/Engine.CharacterMovementComponent|SetGravityScale (Variables|/Script/Engine.Character|GetCharacterMovement _pc_toy) 1.25)
    (Collision|SetActorEnableCollision SelfActor false)
    (Utilities|Time|SetTimerbyFunctionName 0 "Smoorth_Teleport" 2.0 true)
    (CallFunction|SmoorthTeleport _pc_toy OtherActor)
    (Default|CallTakePossession)
    (else
      ;;[0.5724 1 0.6015] Encre a interrupteur
      (if (Actor|ActorHasTag OtherActor "Interupteur")
        (Physics|SetEnableGravity _cube false)
        (Physics|SetPhysicsLinearVelocity _cube "0, 0, 0" false "None")
        (Collision|SetActorEnableCollision OtherActor false)
        (Physics|SetSimulatePhysics _cube false)
        (Variables|Default|SetEstColeeMur true)))))

(event Custom|Smoorth_Teleport
  (params (Tooy :type Actor%20Object%20Reference) (Ennemi :type Actor%20Object%20Reference))
  (bind _returnvalue (Game|GetPlayerController 0))
  (bind _returnvalue_2 (Transformation|GetActorTransform Tooy))
  ;[1 1 1] SmoothTpTransition
  (Variables|Default|SetVeloAvantSmooth (Transformation|GetVelocity Tooy))
  (Input|SetIgnoreMoveInput _returnvalue true)
  (Input|SetIgnoreLookInput _returnvalue true)
  (Collision|SetActorEnableCollision false)
  (Physics|SetPhysicsLinearVelocity (Variables|Default|GetCube) "0, 0, 0" false "None")
  (Components|Movement|StopMovementImmediately (Pawn|GetMovementComponent (Variables|/Script/Engine.Actor|GetInstigator Tooy)))
  (Collision|SetActorEnableCollision Tooy false)
  (Collision|SetActorEnableCollision Ennemi false)
  (Components|Timeline|SetNewTime (Variables|Default|GetSmoothTp) (Variables|Default|GetNew%20Time))
  (bind _returnvalue_3 (Effects|SpawnEmitteratLocation "/Game/NePasToucher/Particles/PC_ParticulesPosses.PC_ParticulesPosses" (.location _returnvalue_2) (.rotation _returnvalue_2) (.scale _returnvalue_2) false))
  (Transformation|SetWorldRotation _returnvalue_3 (Math|Rotator|FindLookatRotation (.location _returnvalue_2) (Transformation|GetActorLocation)) false false)
  (bind _newtrack_0 (Timeline|SmoothTp Play)
    (:Update
      (Transformation|SetActorLocation Tooy (Math|Interpolation|VInterpTo (Transformation|GetActorLocation Tooy) (Transformation|GetActorLocation Ennemi) (- _newtrack_0 (Variables|Default|GetTimeElapsed)) 1e+01) false false)
      (Pawn|SetControlRotation (Pawn|GetController (Variables|/Script/Engine.Actor|GetInstigator Tooy)) (Math|Interpolation|RInterpTo (Transformation|GetActorRotation Tooy) (Transformation|GetActorRotation Ennemi) (- _newtrack_0 (Variables|Default|GetTimeElapsed)) 5.0))
      (Variables|Default|SetTimeElapsed _newtrack_0))
    (:Finished
      (Input|SetIgnoreLookInput _returnvalue false)
      (Variables|/Script/Engine.MovementComponent|SetVelocity (Pawn|GetMovementComponent (Variables|Default|GetPC%20Toy)) (Math|Vector|MakeVector (.x (Math|Vector|RotateVector (* (Math|Vector|MakeVector (+ (Math|Float|Absolute(Float) (.x (Variables|Default|GetVeloAvantSmooth))) (Math|Float|Absolute(Float) (.y (Variables|Default|GetVeloAvantSmooth))) (Math|Float|Absolute(Float) (.z (Variables|Default|GetVeloAvantSmooth)))) 1.0 1.0) (Variables|Default|GetGD_MultiplicationVeloMechaPortal)) (Transformation|GetActorRotation (stale Custom|OnActorHit_Event OtherActor)))) (.y (Math|Vector|RotateVector (* (Math|Vector|MakeVector (+ (Math|Float|Absolute(Float) (.x (Variables|Default|GetVeloAvantSmooth))) (Math|Float|Absolute(Float) (.y (Variables|Default|GetVeloAvantSmooth))) (Math|Float|Absolute(Float) (.z (Variables|Default|GetVeloAvantSmooth)))) 1.0 1.0) (Variables|Default|GetGD_MultiplicationVeloMechaPortal)) (Transformation|GetActorRotation (stale Custom|OnActorHit_Event OtherActor)))) (.z (Math|Vector|RotateVector (* (Math|Vector|MakeVector (+ (Math|Float|Absolute(Float) (.x (Variables|Default|GetVeloAvantSmooth))) (Math|Float|Absolute(Float) (.y (Variables|Default|GetVeloAvantSmooth))) (Math|Float|Absolute(Float) (.z (Variables|Default|GetVeloAvantSmooth)))) 1.0 1.0) (Variables|Default|GetGD_MultiplicationVeloMechaPortal)) (Transformation|GetActorRotation (stale Custom|OnActorHit_Event OtherActor))))))
      (Actor|DestroyActor (stale Custom|OnActorHit_Event OtherActor))
      (Input|SetIgnoreMoveInput _returnvalue false)
      (Input|SetIgnoreLookInput _returnvalue false)
      (Collision|SetActorEnableCollision (Variables|Default|GetPC%20Toy) true)
      (Actor|DestroyActor))))

(event EventBeginPlay
  ;[1 1 1] Tp du joueur sur l'ennemi
  ;;[0.4417 0.5036 1] TP Joueur
  (Variables|Default|SetPC%20Toy (Game|GetPlayerCharacter 0))
  (Collision|SetCollisionObjectType (Variables|Default|GetCube) "ECC_GameTraceChannel1")
  (Variables|Default|SetEstColeeMur false)
  (EventDispatchers|BindEventtoOnActorHit (delegate Custom|OnActorHit_Event))
  (Physics|SetSimulatePhysics (Variables|Default|GetCube) true)
  (Variables|Default|SetReachedTravelTime false)
  ;[1 1 1] Lancement de l'epee
  (Physics|AddForce (Variables|Default|GetCube) (* (Math|Vector|GetUnitDirection(Vector) (Transformation|GetActorLocation (Variables|Default|GetPC%20Toy)) (Transformation|GetActorLocation)) 500000 (Variables|Default|GetGD_ForceLancer)) "None" false)
  ;[1 1 1] Delay avant que l'epee revienne
  (Utilities|FlowControl|Delay (Variables|Default|GetGD_TempsTravelAvantTP))
  (if (not (Variables|Default|GetEstColeeMur))
    (Variables|Default|SetReachedTravelTime true)))

(event EventTick
  (params (DeltaSeconds :type Float%20%28single-precision%29))
  (bind _cube (Variables|Default|GetCube))
  (bind _pc_toy (Variables|Default|GetPC%20Toy))
  (bind _gd_speedepeerevenir (Variables|Default|GetGD_SpeedEpeeRevenir))
  (bind _cube_2 (Variables|Default|GetCube))
  (bind _returnvalue (Transformation|GetActorLocation _pc_toy))
  (bind _returnvalue_2 (Transformation|GetWorldLocation _cube_2))
  (bind _returnvalue_3 (Math|Interpolation|VInterpTo _returnvalue_2 _returnvalue DeltaSeconds _gd_speedepeerevenir))
  (bind _returnvalue_4 (- _returnvalue_3 _returnvalue))
  ;[1 1 1] Epee revenir
  (if (Variables|Default|GetReachedTravelTime)
    (Physics|SetEnableGravity (Variables|Default|GetCube) false)
    (Collision|SetActorEnableCollision false)
    (Physics|SetSimulatePhysics (Variables|Default|GetCube self) false)
    (Physics|SetPhysicsLinearVelocity _cube "0, 0, 0" false "None")
    (Transformation|SetWorldLocation _cube _returnvalue_3 true false)
    (if (< (+ (Math|Float|Absolute(Float) (.x _returnvalue_4)) (Math|Float|Absolute(Float) (.y _returnvalue_4)) (Math|Float|Absolute(Float) (.z _returnvalue_4))) (Variables|Default|GetGD_RangeRecupEpee))
      (Actor|DestroyActor))))

(fn ConstructionScript)