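; BP_Fantome is a ghost system that records the player's path during a run and replays it.
; Tick appends the player's location while EstEnRun is true.
; CoursPetitFantome spawns a collisionless, custom-depth BP_EnnemiTestTP and moves it along a supplied path using a DoN loop, Timeline-driven VInterpTo and delays.
; Record copies the current level's ghost array from the Time game instance into the matching Level variable.
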(event Custom|CoursPetitFantome
  (params (Parcours :type Array%20of%20Vectors))
  (Variables|Default|SetParcoursFantome Parcours)
  (Utilities|FlowControl|Delay 0.25)
  (Variables|Default|SetEstEnRun false)
  (bind _returnvalue (Game|SpawnActorfromClass "/Game/NePasToucher/GameObject/BP_EnnemiTestTP.BP_EnnemiTestTP_C" (Math|Transform|MakeTransform (Utilities|Array|Get(acopy) (Variables|Default|GetParcoursFantome)) "0, 0, 0" "1.000000,1.000000,1.000000") "Undefined" 0 0))
  (bind _output_get (Variables|Default|SetPetitFantome _returnvalue))
  (Rendering|SetRenderCustomDepth (Variables|/Game/NePasToucher/GameObject/BP_EnnemiTestTP.BP_EnnemiTestTP_C|GetCube _output_get) true)
  (Collision|SetActorEnableCollision _output_get false)
  (bind _counter (Utilities|FlowControl|DoN (- (Utilities|Array|Length (Variables|Default|GetParcoursFantome)) 3) :!label _label)
    (:Exit
      (Components|Timeline|SetNewTime (Variables|Default|GetTimeline) 0.0)
      (bind _newtrack_0 (Timeline|Timeline Play)
        (:Update
          (Transformation|SetActorLocation (Variables|Default|GetPetitFantome) (Math|Interpolation|VInterpTo (Utilities|Array|Get(acopy) (Variables|Default|GetParcoursFantome) _counter) (Utilities|Array|Get(acopy) (Variables|Default|GetParcoursFantome) (+ _counter 1)) _newtrack_0 1.0) false false)
          (Utilities|FlowControl|Delay 0.25)
          (if (not (== _counter (- (Utilities|Array|Length (Variables|Default|GetParcoursFantome)) 3)))
            (goto _label)))))))

(event EventTick
  (params (DeltaSeconds :type Float%20%28single-precision%29))
  (if (Variables|Default|GetEstEnRun)
    (Utilities|Array|Add (Variables|Default|GetParcoursFantome) (Transformation|GetActorLocation (Game|GetPlayerCharacter 0)))))

(fn ConstructionScript)

(fn Record
  (bind _astime (Utilities|Casting|CastToTime (Game|GetGameInstance)))
  (switch int (Variables|/Game/Teliau/Blueprint/Time.Time_C|GetCurrenteLevel _astime)
    (:0
      (Variables|Default|SetLevel0 (Variables|/Game/Teliau/Blueprint/Time.Time_C|GetArrayPetitFantome1 _astime)))
    (:1
      (Variables|Default|SetLevel1 (Variables|/Game/Teliau/Blueprint/Time.Time_C|GetArrayPetitFantome2 _astime)))
    (:2
      (Variables|Default|SetLevel2 (Variables|/Game/Teliau/Blueprint/Time.Time_C|GetArrayPetitFantome3 _astime)))
    (:3
      (Variables|Default|SetLevel3 (Variables|/Game/Teliau/Blueprint/Time.Time_C|GetArrayPetitFantome4 _astime)))))