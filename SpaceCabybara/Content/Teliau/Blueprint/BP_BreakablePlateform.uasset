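; BP_BreakablePlateform is a platform that breaks after the player's toy character hits it, then respawns.
; A hit on the Cylinder from a PC_ToyCharacter swaps its material as a warning, then hides it and disables its collision after Duration.
; After DurationRespawn it restores visibility, collision and the BasicShapeMaterial material, all through a simple Delay chain in the event graph.
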(event OnComponentHit(Cylinder)
  (params (HitComponent :type Primitive%20Component%20Object%20Reference) (OtherActor :type Actor%20Object%20Reference) (OtherComp :type Primitive%20Component%20Object%20Reference) (NormalImpulse :type Vector :default "0, 0, 0") (Hit :type Hit%20Result%20Structure%20%28by%20ref%29))
  (Utilities|Casting|CastToPC_ToyCharacter OtherActor)
  (Rendering|Material|SetMaterial (Variables|Default|GetCylinder) 0 "/Engine/MapTemplates/Materials/BasicAsset03.BasicAsset03")
  (Utilities|FlowControl|Delay (Variables|Default|GetDuration))
  (Rendering|SetVisibility (Variables|Default|GetCylinder) false false)
  (Collision|SetCollisionEnabled (Variables|Default|GetCylinder) "NoCollision")
  (Utilities|FlowControl|Delay (Variables|Default|GetDurationRespawn))
  (Rendering|SetVisibility (Variables|Default|GetCylinder) true false)
  (Collision|SetCollisionEnabled (Variables|Default|GetCylinder) "QueryAndPhysics")
  (Rendering|Material|SetMaterial (Variables|Default|GetCylinder) 0 "/Engine/BasicShapes/BasicShapeMaterial.BasicShapeMaterial"))

(fn ConstructionScript)