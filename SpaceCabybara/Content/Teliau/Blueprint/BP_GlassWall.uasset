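; BP_GlassWall is a breakable glass wall that the toy character can smash through.
; When its box component is overlapped, it casts the other actor to PC_ToyCharacter and checks the IsHulkSmashing flag.
; If the flag is set, it plays a glass-break sound with randomized volume and pitch, then destroys itself.
; Debug strings print the touch and the flag's value.
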(event OnComponentBeginOverlap(Box)
  (params (OverlappedComponent :type Primitive%20Component%20Object%20Reference) (OtherActor :type Actor%20Object%20Reference) (OtherComp :type Primitive%20Component%20Object%20Reference) (OtherBodyIndex :type Integer) (bFromSweep :type Boolean) (SweepResult :type Hit%20Result%20Structure%20%28by%20ref%29))
  (Development|PrintString "Touched")
  (bind _aspc_toy_character (Utilities|Casting|CastToPC_ToyCharacter OtherActor))
  (Development|PrintString (Utilities|String|ToString(Boolean) (Variables|/Game/NePasToucher/GameObject/PC_ToyCharacter.PC_ToyCharacter_C|GetIsHulkSmashing _aspc_toy_character)))
  (if (Variables|/Game/NePasToucher/GameObject/PC_ToyCharacter.PC_ToyCharacter_C|GetIsHulkSmashing _aspc_toy_character)
    (Audio|PlaySoundatLocation "/Game/Teliau/Sound/glass-break-1-80963.glass-break-1-80963" (Transformation|GetActorLocation) "0, 0, 0" (Math|Random|RandomFloatinRange 0.8 5.0) (Math|Random|RandomFloatinRange 0.8 5.0) 0.0 0 0 0 0)
    (Actor|DestroyActor)))

(fn ConstructionScript)