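; BP_Bumper is a bumper pad that launches a PC_ToyCharacter upward when it overlaps the Box trigger.
; At BeginPlay it caches Cube1's relative transform and a copy raised by HauteurPlateform.
; On overlap it prints a debug string, waits for Duration, then launches the character with vertical Force.
; A Timeline started alongside the launch lerps Cube1 between the two cached transforms to animate the bump.
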(event OnComponentBeginOverlap(Box)
  (params (OverlappedComponent :type Primitive%20Component%20Object%20Reference) (OtherActor :type Actor%20Object%20Reference) (OtherComp :type Primitive%20Component%20Object%20Reference) (OtherBodyIndex :type Integer) (bFromSweep :type Boolean) (SweepResult :type Hit%20Result%20Structure%20%28by%20ref%29))
  (bind _aspc_toy_character (Utilities|Casting|CastToPC_ToyCharacter OtherActor))
  (Development|PrintString "Hello")
  (Utilities|FlowControl|Delay (Variables|Default|GetDuration))
  (Utilities|FlowControl|Sequence
    (:then_0
      (Character|LaunchCharacter _aspc_toy_character (Math|Vector|MakeVector 0.0 0.0 (Variables|Default|GetForce)) false false))
    (:then_1
      (bind _newtrack_0 (Timeline|Timeline PlayFromStart)
        (:Update
          (Transformation|SetRelativeTransform (Variables|Default|GetCube1) (Math|Transform|Lerp(Transform) (Variables|Default|GetPositionBumperInit) (Variables|Default|GetPositionBumperThen) _newtrack_0) false false))))))

(event EventBeginPlay
  (bind _cube1 (Variables|Default|GetCube1))
  (bind _returnvalue (Transformation|GetRelativeTransform _cube1))
  (bind (_location _rotation _scale) (Math|Transform|BreakTransform _returnvalue))
  (Variables|Default|SetPositionBumperInit _returnvalue)
  (Variables|Default|SetPositionBumperThen (Math|Transform|MakeTransform (Math|Vector|MakeVector (.x _location) (.y _location) (+ (.z _location) (Variables|Default|GetHauteurPlateform))) _rotation _scale)))

(fn ConstructionScript)