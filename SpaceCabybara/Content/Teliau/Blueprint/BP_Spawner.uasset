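; One-shot enemy spawner that fires when the PC_ToyCharacter enters its Box trigger.
; At BeginPlay, a GDShootSpawner flag picks either AI_Ennemi with BT_EnnemyBrain or AI_EnnemiRun with BT_EnnemyBrainRun.
; On overlap, it loops on NombreDeMechants, spawning AI at random XY offsets sized by Box1's extent around the Scene component, then destroys itself.
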(event OnComponentBeginOverlap(Box)
  (params (OverlappedComponent :type Primitive%20Component%20Object%20Reference) (OtherActor :type Actor%20Object%20Reference) (OtherComp :type Primitive%20Component%20Object%20Reference) (OtherBodyIndex :type Integer) (bFromSweep :type Boolean) (SweepResult :type Hit%20Result%20Structure%20%28by%20ref%29))
  (bind _box1 (Variables|Default|GetBox1))
  (bind _scene (Variables|Default|GetScene))
  (bind _returnvalue (Transformation|GetWorldTransform _scene))
  (bind _returnvalue_2 (Components|Box|GetScaledBoxExtent _box1))
  (bind (_x _y) (Math|Vector|BreakVector _returnvalue_2))
  (bind (_location _rotation) (Math|Transform|BreakTransform _returnvalue))
  (Utilities|Casting|CastToPC_ToyCharacter OtherActor)
  (for _index (range 0 (Variables|Default|GetNombre%20de%20Mechants))
    (AI|SpawnAIFromClass (Variables|Default|GetPawn%20Class) (Variables|Default|GetBehavior%20Tree) (+ _location (Math|Vector|MakeVector (Math|Random|RandomFloatinRange (* -1 _x) _x) (Math|Random|RandomFloatinRange (* -1 _y) _y) 0.0)) _rotation false 0))
  (Actor|DestroyActor))

(event EventBeginPlay
  (if (Variables|Default|GetGD_ShootSpawner)
    (Variables|Default|SetPawn%20Class "/Game/Teliau/Blueprint/IA/AI_Ennemi.AI_Ennemi_C")
    (Variables|Default|SetBehavior%20Tree "/Game/Teliau/Blueprint/IA/BT_EnnemyBrain.BT_EnnemyBrain")
    (else
      (Variables|Default|SetPawn%20Class "/Game/Teliau/Blueprint/IA/AI_EnnemiRun.AI_EnnemiRun_C")
      (Variables|Default|SetBehavior%20Tree "/Game/Teliau/Blueprint/IA/BT_EnnemyBrainRun.BT_EnnemyBrainRun"))))

(fn ConstructionScript)