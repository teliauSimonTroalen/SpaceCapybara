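; Bullet is a physics-driven projectile actor that triggers a death call when it hits the toy character.
; On BeginPlay it launches its Sphere with the Impulse variable and destroys itself after a short delay.
; A Sphere hit on PC_ToyCharacter calls Meurs on the first UltimateBlueprintMasterDeluxe found in the level, then destroys the bullet immediately; other hits are ignored.
; An unconnected swept-movement chain remains in the graph and never runs.
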(event OnComponentHit(Sphere)
  (params (HitComponent :type Primitive%20Component%20Object%20Reference) (OtherActor :type Actor%20Object%20Reference) (OtherComp :type Primitive%20Component%20Object%20Reference) (NormalImpulse :type Vector :default "0, 0, 0") (Hit :type Hit%20Result%20Structure%20%28by%20ref%29))
  (Utilities|Casting|CastToPC_ToyCharacter OtherActor)
  (bind _outactors (Actor|GetAllActorsOfClass "/Game/Teliau/Blueprint/UltimateBlueprintMasterDeluxe.UltimateBlueprintMasterDeluxe_C"))
  (Default|Meurs (Utilities|Array|Get(acopy) _outactors))
  (Actor|DestroyActor))

(event EventBeginPlay
  (Physics|AddImpulse (Variables|Default|GetSphere) (Variables|Default|GetImpulse) "None" false)
  (Utilities|FlowControl|Delay 5.0)
  (Actor|DestroyActor))

(event EventTick
  (params (DeltaSeconds :type Float%20%28single-precision%29)))

(fn ConstructionScript)