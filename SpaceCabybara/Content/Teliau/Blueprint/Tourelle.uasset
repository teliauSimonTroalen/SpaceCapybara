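; Turret actor that turns in fixed angular steps and fires a Bullet at regular intervals.
; Tick uses the IsSpinning flag and a short Delay as a cooldown gate, so each step runs about twice per second.
; Each step rotates the actor, then spawns a Bullet at its location, with rotation offset from the new facing by another step plus a quarter turn.
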(event EventTick
  (params (DeltaSeconds :type Float%20%28single-precision%29))
  (if (not (Variables|Default|GetIsSpinning))
    (Variables|Default|SetIsSpinning true)
    (Transformation|SetActorRotation (Math|Rotator|CombineRotators (Transformation|GetActorRotation) "0.000000,10.000000,0.000000"))
    (Game|SpawnActorfromClass "/Game/Teliau/Blueprint/Bullet.Bullet_C" (Math|Transform|MakeTransform (Transformation|GetActorLocation) (Math|Rotator|CombineRotators (Math|Rotator|CombineRotators (Transformation|GetActorRotation) "0.000000,10.000000,0.000000") "90.000000,0.000000,0.000000")) "Undefined" 0 0)
    (Utilities|FlowControl|Delay 0.5)
    (Variables|Default|SetIsSpinning false)))

(fn ConstructionScript)