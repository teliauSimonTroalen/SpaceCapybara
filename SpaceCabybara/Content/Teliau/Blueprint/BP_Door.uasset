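; Interactable sliding door that toggles between its initial position and an end position offset by configurable X, Y and Z values.
; BeginPlay caches both positions from the mesh's world location, and Interact flips the open state and plays the matching timeline.
; Each timeline moves the scene root by lerping from the mesh's current location, not a fixed start.
; Interacting mid-movement stops both timelines and reverses direction.
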(event EventInteract
  (bind _defaultsceneroot (Variables|Default|GetDefaultSceneRoot))
  (if (Variables|Default|GetisMoving)
    (Utilities|FlowControl|Sequence
      (:then_0
        (bind _newtrack_0 (Timeline|Timeline Stop)
          (:Update
            (Transformation|SetWorldLocation _defaultsceneroot (Math|Vector|Lerp(Vector) (Transformation|GetWorldLocation (Variables|Default|GetStaticMesh)) (Variables|Default|GetPosition_End) _newtrack_0) false false))
          (:Finished
            (Development|PrintString "J'ai fini de bouger" :!label _label)
            (Variables|Default|SetisMoving false))))
      (:then_1
        (bind _newtrack_0_2 (Timeline|Timeline_0 Stop)
          (:Update
            (Transformation|SetWorldLocation _defaultsceneroot (Math|Vector|Lerp(Vector) (Transformation|GetWorldLocation (Variables|Default|GetStaticMesh)) (Variables|Default|GetPosition_Init) _newtrack_0_2) false false))
          (:Finished
            (goto _label))))
      (:then_2
        (if (not (Variables|Default|GetisOpen)) :!label _label_2
          (Variables|Default|SetisMoving true)
          (Variables|Default|SetisOpen true)
          (Timeline|Timeline PlayFromStart)
          (else
            (Variables|Default|SetisMoving true)
            (Variables|Default|SetisOpen false)
            (Timeline|Timeline_0 PlayFromStart)))))
    (else
      (goto _label_2))))

(event EventBeginPlay
  (bind _staticmesh (Variables|Default|GetStaticMesh))
  (bind _returnvalue (Transformation|GetWorldLocation _staticmesh))
  (bind (_x _y _z) (Math|Vector|BreakVector _returnvalue))
  (Variables|Default|SetPosition_Init _returnvalue)
  (Variables|Default|SetPosition_End (Math|Vector|MakeVector (+ _x (Variables|Default|GetX_Value)) (+ _y (Variables|Default|GetY_Value)) (+ _z (Variables|Default|GetZ_Value)))))

(fn ConstructionScript)