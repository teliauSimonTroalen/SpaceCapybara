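; Behavior Tree task that makes an AI_Ennemi pawn fire Bullet projectiles.
; On execute it starts a looping timer at a random interval, which the task never clears.
; Each Shoot plays MonsterBeam with random volume and pitch, spawns a Bullet at ShootFrom with a forward impulse, then finishes the task successfully.
; A visibility line trace meant to gate firing is left disconnected.
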(event Custom|Shoot
  (Audio|PlaySoundatLocation "/Game/Teliau/Sound/MonsterBeam.MonsterBeam" (Transformation|GetWorldLocation (Variables|/Game/Teliau/Blueprint/IA/AI_Ennemi.AI_Ennemi_C|GetShootFrom (stale EventReceiveExecuteAI _asai_ennemi))) "0, 0, 0" (Math|Random|RandomFloatinRange 0.2 0.5) (Math|Random|RandomFloatinRange 1.0 1e+01) 0.0 0 0 0 0)
  (Game|SpawnActorfromClass "/Game/Teliau/Blueprint/Bullet.Bullet_C" (Math|Transform|MakeTransform (Transformation|GetWorldLocation (Variables|/Game/Teliau/Blueprint/IA/AI_Ennemi.AI_Ennemi_C|GetShootFrom (stale EventReceiveExecuteAI _asai_ennemi)))) "Undefined" 0 (* (Math|Vector|GetForwardVector (Variables|/Game/Teliau/Blueprint/IA/AI_Ennemi.AI_Ennemi_C|GetShootFrom (stale EventReceiveExecuteAI _asai_ennemi))) 1e+03) 0)
  (AI|BehaviorTree|FinishExecute true))

(event EventReceiveExecuteAI
  (params (OwnerController :type AI%20Controller%20Object%20Reference) (ControlledPawn :type Pawn%20Object%20Reference))
  (bind _asai_ennemi (Utilities|Casting|CastToAI_Ennemi ControlledPawn))
  (Utilities|Time|SetTimerbyEvent (delegate Custom|Shoot) (Math|Random|RandomFloatinRange 0.1 1.2) true))