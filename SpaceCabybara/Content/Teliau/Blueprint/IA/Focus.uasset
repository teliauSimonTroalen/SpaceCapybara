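; Behavior tree task that makes an AI_Ennemi aim and focus on player 0.
; It sets the relative pitch of the enemy's ShootFrom component from the arcsine of the height difference to the player's capsule over the actor-to-actor distance, zeroing roll and yaw.
; The AI controller then sets focus on the player, and the task finishes successfully.
; An alternative world-rotation version of the aim is left disconnected.
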(event EventReceiveExecuteAI
  (params (OwnerController :type AI%20Controller%20Object%20Reference) (ControlledPawn :type Pawn%20Object%20Reference))
  (bind _returnvalue (Game|GetPlayerCharacter 0))
  (bind _asennemi (Utilities|Casting|CastToAI_Ennemi ControlledPawn))
  (Transformation|SetRelativeRotation (Variables|/Game/Teliau/Blueprint/IA/AI_Ennemi.AI_Ennemi_C|GetShootFrom _asennemi) (Math|Rotator|MakeRotator 0.0 (Class|KismetMathLibrary|DegAsin (/ (- (.z (Transformation|GetWorldLocation (Variables|/Script/Engine.Character|GetCapsuleComponent _returnvalue))) (.z (Transformation|GetWorldLocation (Variables|/Game/Teliau/Blueprint/IA/AI_Ennemi.AI_Ennemi_C|GetShootFrom _asennemi)))) (Transformation|GetDistanceTo _returnvalue _asennemi))) 0.0) false false)
  (AI|SetFocus OwnerController _returnvalue)
  (AI|BehaviorTree|FinishExecute true))