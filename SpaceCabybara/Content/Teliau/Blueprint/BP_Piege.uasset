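; BP_Piege is a trap that swings two arrow components when a PC_ToyCharacter enters its box collision.
; BeginPlay caches both arrows' world rotations and derives end rotations by adding a pitch offset.
; On overlap, a timeline lerps both from start to end, applying the values as relative rotations.
; When the timeline finishes, it calls TuMeursMartoniLaRevancheLaRevanche, whose handling is outside this graph.
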(event OnComponentBeginOverlap(BoxCollision)
  (params (OverlappedComponent :type Primitive%20Component%20Object%20Reference) (OtherActor :type Actor%20Object%20Reference) (OtherComp :type Primitive%20Component%20Object%20Reference) (OtherBodyIndex :type Integer) (bFromSweep :type Boolean) (SweepResult :type Hit%20Result%20Structure%20%28by%20ref%29))
  (Development|PrintString "Hello")
  (Utilities|Casting|CastToPC_ToyCharacter OtherActor)
  (bind _newtrack_0 (Timeline|Timeline PlayFromStart)
    (:Update
      (Transformation|SetRelativeRotation (Variables|Default|GetArrowR) (Math|Rotator|Lerp(Rotator) (Variables|Default|GetRotation%20InitR) (Variables|Default|GetRotation%20EndR) _newtrack_0) false false)
      (Transformation|SetRelativeRotation (Variables|Default|GetArrowL) (Math|Rotator|Lerp(Rotator) (Variables|Default|GetRotation%20InitL) (Variables|Default|GetRotation%20EndL) _newtrack_0) false false))
    (:Finished
      (Default|CallTuMeursMartoniLaRevancheLaRevanche))))

(event EventBeginPlay
  (bind _output_get (Variables|Default|SetRotation%20InitR (Transformation|GetWorldRotation (Variables|Default|GetArrowR))))
  (bind _output_get_2 (Variables|Default|SetRotation%20InitL (Transformation|GetWorldRotation (Variables|Default|GetArrowL))))
  (Variables|Default|SetRotation%20EndR (Math|Rotator|MakeRotator (.Roll (Math|Rotator|BreakRotator _output_get)) (+ (.Pitch (Math|Rotator|BreakRotator _output_get)) (Variables|Default|GetRotation%20Additivite)) (.Yaw (Math|Rotator|BreakRotator _output_get))))
  (Variables|Default|SetRotation%20EndL (Math|Rotator|MakeRotator (.Roll (Math|Rotator|BreakRotator _output_get_2)) (+ (.Pitch (Math|Rotator|BreakRotator _output_get_2)) (Variables|Default|GetRotation%20Additivite)) (.Yaw (Math|Rotator|BreakRotator _output_get_2)))))

(fn ConstructionScript)