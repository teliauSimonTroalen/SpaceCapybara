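; Central level manager that wires fragment pickups, traps, death zones, checkpoints, the end zone and the pause menu through event bindings.
; Collecting every memory fragment triggers the final door; death teleports the player to the last checkpoint and respawns destroyed "Destruisible" actors from saved transforms.
; Tick drives a gated run timer and a looping ten-second gauge, reset by sword possession.
; Finishing stores time and level name in the GameInstance, then opens LevelFin.
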(event Custom|AugmenterLeScore
  (bind _output_get (Variables|Default|SetNouveau%20Score (+ (Variables|Default|GetNouveau%20Score) 1)))
  (Default|DisplayScore (Variables|/Game/NePasToucher/Game/PC_ToyController.PC_ToyController_C|GetWidgetInterface (Utilities|Array|Get(acopy) (stale EventBeginPlay _outactors_2))) _output_get)
  (if (>= (Variables|Default|GetNouveau%20Score) (Utilities|Array|Length (stale EventBeginPlay _outactors)))
    (bind _outactors (Actor|GetAllActorsOfClass "/Game/Teliau/Blueprint/BP_Door.BP_Door_C"))
    (for _array_element _outactors
      (if (Actor|ActorHasTag _array_element "Finale_Door")
        (Default|Interact _array_element)))))

(event Custom|TuMeurs
  (CallFunction|Meurs))

(event Custom|Tu%20Checkpointes
  (params (CheckPointEnQuestion :type BP%20Zone%20De%20Check%20Point%20Object%20Reference))
  (Variables|Default|SetTempusFugit 0.0)
  (Variables|Default|SetLastCheckPoint CheckPointEnQuestion)
  (Utilities|Array|Clear (Variables|Default|GetEnnemis))
  (bind _outactors (Actor|GetAllActorswithTag "Destruisible"))
  (bind _output_get (Variables|Default|SetEnnemis _outactors))
  (Utilities|Array|Clear (Variables|Default|GetEnnemisTransform))
  (for _array_element _output_get
    (bind _returnvalue (Utilities|Array|Add (Variables|Default|GetEnnemisTransform) (Transformation|GetActorTransform _array_element)))))

(event Custom|StartTimer
  (Utilities|FlowControl|Gate true) ; enters at Open
)

(event Custom|StopTimer
  (Utilities|FlowControl|Gate true) ; enters at Close
)

(event Custom|ResetTempusFugit
  (Variables|Default|SetTempusFugit 0.0)
  (Default|DisplaySpareTime (Variables|/Game/NePasToucher/Game/PC_ToyController.PC_ToyController_C|GetWidgetInterface (Utilities|Array|Get(acopy) (stale EventBeginPlay _outactors_2))) 0.0))

(event Custom|Finis
  (bind _astime (Utilities|Casting|CastToTime (Game|GetGameInstance)))
  (Variables|/Game/Teliau/Blueprint/Time.Time_C|SetInstanceSecondes _astime (Variables|Default|GetSecondes))
  (Variables|/Game/Teliau/Blueprint/Time.Time_C|SetInstannceMinutes _astime (Variables|Default|GetMinutes))
  (Variables|/Game/Teliau/Blueprint/Time.Time_C|SetInstanceCentiemes _astime (Variables|Default|GetCentieme))
  (bind _returnvalue (Game|GetCurrentLevelName true))
  (Variables|/Game/Teliau/Blueprint/Time.Time_C|SetNamePastLevel _astime (Utilities|String|StringToName _returnvalue))
  (Game|OpenLevel(byName) (Variables|Default|GetLevelFin)))

(event EventTick
  (params (DeltaSeconds :type Float%20%28single-precision%29))
  (Utilities|FlowControl|Sequence
    (:then_0
      (Default|DisplaySpareTime (Variables|/Game/NePasToucher/Game/PC_ToyController.PC_ToyController_C|GetWidgetInterface (Utilities|Array|Get(acopy) (stale EventBeginPlay _outactors_2))) (/ (Variables|Default|GetTempusFugit) 1e+01))
      (Variables|Default|SetTempusFugit (+ (Variables|Default|GetTempusFugit) DeltaSeconds))
      (if (>= (Variables|Default|GetTempusFugit) 1e+01)
        (Variables|Default|SetTempusFugit 0.0)))
    (:then_1
      (Utilities|FlowControl|Gate true
        (:Exit
          (Default|DisplayTime (Variables|/Game/NePasToucher/Game/PC_ToyController.PC_ToyController_C|GetWidgetInterface (Utilities|Array|Get(acopy) (stale EventBeginPlay _outactors_2))) (Variables|Default|GetMinutes) (Variables|Default|GetSecondes) (Variables|Default|GetCentieme))
          (Variables|Default|SetCentieme (+ (Variables|Default|GetCentieme) DeltaSeconds))
          (if (> (Variables|Default|GetCentieme) 0.99)
            (Variables|Default|SetCentieme 0.0)
            (Variables|Default|SetSecondes (+ (Variables|Default|GetSecondes) 1))
            (if (> (Variables|Default|GetSecondes) 59)
              (Variables|Default|SetSecondes 0)
              (Variables|Default|SetMinutes (+ (Variables|Default|GetMinutes) 1)))))))
    (:then_2
      (bind _outactors (Actor|GetAllActorsOfClass "/Game/NePasToucher/GameObject/PC_Epee.PC_Epee_C"))
      (if (Utilities|IsValid (Utilities|Array|Get(acopy) _outactors))
        (EventDispatchers|BindEventtoTakePossession (Utilities|Array|Get(acopy) _outactors) (delegate Custom|ResetTempusFugit))))))

(event EventBeginPlay
  (Utilities|FlowControl|Sequence
    (:then_0
      (bind _outactors (Actor|GetAllActorsOfClass "/Game/Teliau/Blueprint/BP_FragmentDeMemoire.BP_FragmentDeMemoire_C"))
      (bind _outactors_2 (Actor|GetAllActorsOfClass "/Game/NePasToucher/Game/PC_ToyController.PC_ToyController_C"))
      (EventDispatchers|BindEventtoRemasserFragmentMemoire _outactors (delegate Custom|AugmenterLeScore))
      (bind _outactors_3 (Actor|GetAllActorsOfClass "/Game/Teliau/Blueprint/BP_Piege.BP_Piege_C"))
      (EventDispatchers|BindEventtoTuMeursMartoniLaRevancheLaRevanche _outactors_3 (delegate Custom|TuMeurs))
      (bind _outactors_4 (Actor|GetAllActorsOfClass "/Game/Teliau/Blueprint/Zones/BP_ZoneDeMort.BP_ZoneDeMort_C"))
      (EventDispatchers|BindEventtoTuMeursMartoni _outactors_4 (delegate Custom|TuMeurs))
      (bind _outactors_5 (Actor|GetAllActorsOfClass "/Game/Teliau/Blueprint/Zones/BP_ZoneDeCheckPoint.BP_ZoneDeCheckPoint_C"))
      (EventDispatchers|BindEventtoTuPassesUnCheckPoint _outactors_5 (delegate Custom|Tu%20Checkpointes))
      (bind _returnvalue (UserInterface|CreateWidget "/Game/Teliau/Blueprint/UI/WI_Pause_Menu.WI_Pause_Menu_C"))
      (bind _output_get (Variables|Default|SetPauseMenu _returnvalue))
      (UserInterface|Viewport|AddtoViewport _output_get 0)
      (Widget|SetVisibility _output_get "Hidden")
      (CallFunction|StartTimer)
      (EventDispatchers|BindEventtoStartTimer (Variables|Default|GetPauseMenu) (delegate Custom|StartTimer))
      (bind _outactors_6 (Actor|GetAllActorsOfClass "/Game/Teliau/Blueprint/Zones/BP_ZoneDeFin.BP_ZoneDeFin_C"))
      (EventDispatchers|BindEventtoZoneDeFin _outactors_6 (delegate Custom|Finis)))
    (:then_1
      (Variables|Default|SetLastCheckPoint (stale Custom|Tu%20Checkpointes CheckPointEnQuestion))
      (Utilities|Array|Clear (Variables|Default|GetEnnemis))
      (bind _outactors_7 (Actor|GetAllActorswithTag "Destruisible"))
      (bind _output_get_2 (Variables|Default|SetEnnemis _outactors_7))
      (Utilities|Array|Clear (Variables|Default|GetEnnemisTransform))
      (for _array_element _output_get_2
        (bind _returnvalue_2 (Utilities|Array|Add (Variables|Default|GetEnnemisTransform) (Transformation|GetActorTransform _array_element)))))))

(event Input|KeyboardEvents|P
  (params (Key :type Key%20Structure :default "None"))
  (bind _returnvalue (Game|GetPlayerController 0))
  (bind _returnvalue_2 (Game|GetPlayerController 0))
  (bind _pausemenu (Variables|Default|GetPauseMenu))
  (:Pressed
    (if true
      (Widget|SetVisibility _pausemenu "Visible")
      (Input|SetInputModeUIOnly _returnvalue 0 "DoNotLock" false)
      (Variables|/Script/Engine.PlayerController|SetbShowMouseCursor _returnvalue true)
      (CallFunction|StopTimer)
      (Variables|Default|SetPaused true)
      (else
        (Widget|SetVisibility _pausemenu "Hidden")
        (Input|SetInputModeGameOnly _returnvalue_2 false)
        (Variables|/Script/Engine.PlayerController|SetbShowMouseCursor _returnvalue_2 false)
        (CallFunction|StartTimer)
        (Variables|Default|SetPaused false)))))

(fn ConstructionScript)

(fn Meurs
  (bind _returnvalue (Game|GetPlayerCharacter 0))
  (bind _lastcheckpoint (Variables|Default|GetLastCheckPoint))
  (bind _arrow (Variables|/Game/Teliau/Blueprint/Zones/BP_ZoneDeCheckPoint.BP_ZoneDeCheckPoint_C|GetArrow _lastcheckpoint))
  (bind _returnvalue_2 (Transformation|GetWorldRotation _arrow))
  (Transformation|Teleport _returnvalue (Transformation|GetWorldLocation _arrow) _returnvalue_2)
  (Pawn|SetControlRotation (Game|GetPlayerController (Variables|/Script/Engine.Pawn|GetPlayerState _returnvalue)) _returnvalue_2)
  (for (_array_element _array_index) (Variables|Default|GetEnnemis)
    (if (not (Utilities|IsValid _array_element))
      (bind _returnvalue_3 (Game|SpawnActorfromClass (Utilities|GetClass _array_element) (Utilities|Array|Get(acopy) (Variables|Default|GetEnnemisTransform) _array_index) "AlwaysSpawn" 0 0))
      (Utilities|Array|SetArrayElem (Variables|Default|GetEnnemis) _array_index _returnvalue_3)))
  (Variables|Default|SetTempusFugit 0.0))