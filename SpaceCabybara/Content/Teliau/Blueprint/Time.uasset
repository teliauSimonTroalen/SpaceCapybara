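; The Time Blueprint holds ghost path data ("CheminPetitFantome") for four levels.
; StockTonFantomeMonPote stores a given path in the ArrayPetitFantome variable selected by the level index.
; DonneMoiMonFantome returns the stored path for a given level index.
; Both functions switch on the index to pick one of four separate variables, one per level.
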(fn DonneMoiMonFantome
  (params (Niveau :type Integer))
  (switch int Niveau ; On lui donne lequel
    (:0
      (return (Variables|Default|GetArrayPetitFantome1)))
    (:1
      (return (Variables|Default|GetArrayPetitFantome2)))
    (:2
      (return (Variables|Default|GetArrayPetitFantome3)))
    (:3
      (return (Variables|Default|GetArrayPetitFantome4)))))

(fn StockTonFantomeMonPote
  (params (Niveau :type Integer) (CheminPetitFantome :type Array%20of%20Vectors))
  (switch int Niveau ; On lui donne lequel
    (:0
      (Variables|Default|SetArrayPetitFantome1 CheminPetitFantome))
    (:1
      (Variables|Default|SetArrayPetitFantome2 CheminPetitFantome))
    (:2
      (Variables|Default|SetArrayPetitFantome3 CheminPetitFantome))
    (:3
      (Variables|Default|SetArrayPetitFantome4 CheminPetitFantome))))