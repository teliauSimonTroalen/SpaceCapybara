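; BP_laser is a moving laser hazard that sets its Niagara beam end from LengthBeam at start.
; Overlapping a PC_ToyCharacter calls Meurs on the UltimateBlueprintMasterDeluxe actor to kill and respawn the player.
; Tick eases the Box toward the current PointsList location with VInterpTo.
; The index only changes at the list's first and last entries, so it ping-pongs with two points but stays on any middle one.
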(event EventBeginPlay
  ;[1 1 1] Value of the beam length
  (Effects|Components|ParticleSystem|SetVectorParameter (Variables|Default|GetNiagara) "Beam End" (Variables|Default|GetLengthBeam)))

(event Collision|EventActorBeginOverlap
  (params (OtherActor :type Actor%20Object%20Reference))
  ;[1 1 1] Kill player and respawn back
  (Utilities|IsValid OtherActor
    (:Is%20Valid
      (Utilities|Casting|CastToPC_ToyCharacter OtherActor)
      (bind _returnvalue (Actor|GetActorOfClass "/Game/Teliau/Blueprint/UltimateBlueprintMasterDeluxe.UltimateBlueprintMasterDeluxe_C"))
      (Default|Meurs _returnvalue))))

(event EventTick
  (params (DeltaSeconds :type Float%20%28single-precision%29))
  (bind _box (Variables|Default|GetBox))
  (bind _returnvalue (Transformation|GetWorldLocation _box))
  (Transformation|SetWorldLocation _box (Math|Interpolation|VInterpTo _returnvalue (Utilities|Array|Get(acopy) (Variables|Default|GetPointsList) (Variables|Default|GetIDPoint)) DeltaSeconds 1.0) false false)
  (if (<= (Math|Vector|Distance(Vector) _returnvalue (Utilities|Array|Get(acopy) (Variables|Default|GetPointsList) (Variables|Default|GetIDPoint))) 1e+01)
    (Utilities|FlowControl|Sequence
      (:then_0
        (if (== (Variables|Default|GetIDPoint) 0)
          (Variables|Default|SetIDPoint (+ (Variables|Default|GetIDPoint) 1))
          (elif (== (Variables|Default|GetIDPoint) (- (Utilities|Array|Length (Variables|Default|GetPointsList)) 1))
            (Variables|Default|SetIDPoint (- (Variables|Default|GetIDPoint) 1)))))
      (:then_1
        (Development|PrintString (Utilities|String|ToString(Integer) (Variables|Default|GetIDPoint)))))))

(fn ConstructionScript)