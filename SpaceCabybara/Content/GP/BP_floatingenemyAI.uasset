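; BP_floatingenemyAI holds the patrol route for a floating enemy, defined by a spline.
; On BeginPlay it caches the world location of each spline point into the PatrolPoint array.
; GetNextLocation steps CurrentPoint through that array, reversing PatrolDir at either end for a back-and-forth patrol, and returns the next location.
; The file only supplies destinations and contains no movement logic.
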(event EventBeginPlay
  (CallFunction|InitialisePatrolPoint))

(fn ConstructionScript)

(fn InitialisePatrolPoint
  (for _index (range 0 (- (Spline|GetNumberOfSplinePoints (Variables|Default|GetSpline)) 1))
    (Utilities|Array|Add (Variables|AI|GetPatrolPoint) (Spline|GetLocationatSplinePoint (Variables|Default|GetSpline) _index "World"))))

(fn GetNextLocation
  (if (< (Variables|Default|GetCurrentPoint) 1)
    (Variables|Default|SetPatrolDir 1)
    (elif (>= (Variables|Default|GetCurrentPoint) (Utilities|Array|LastIndex (Variables|AI|GetPatrolPoint)))
      (Variables|Default|SetPatrolDir -1)))
  (Variables|Default|SetCurrentPoint (+ (Variables|Default|GetPatrolDir) (Variables|Default|GetCurrentPoint)))
  (return (Utilities|Array|Get(acopy) (Variables|AI|GetPatrolPoint) (Variables|Default|GetCurrentPoint))))