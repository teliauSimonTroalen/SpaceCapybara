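; BP_puppet is a character Blueprint that implements wall running while airborne.
; Each falling tick, visibility line traces probe right and left, gated by side flags, with debug drawing.
; A hit, unless jumping off, aligns yaw to the wall normal and zeroes gravity, setting forward velocity on the right but zero velocity on the left.
; A miss calls OffWall to restore gravity.
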(event Custom|OffWall
  (bind _charactermovement (Variables|Character|GetCharacterMovement))
  (Variables|/Script/Engine.CharacterMovementComponent|SetGravityScale _charactermovement 1.0)
  (Class|MovementComponent|SetPlaneConstraintNormal _charactermovement "0, 0, 0"))

(event EventBeginPlay
  (Class|MovementComponent|SetPlaneConstraintEnabled (Variables|Character|GetCharacterMovement) false))

(event EventTick
  (params (DeltaSeconds :type Float%20%28single-precision%29))
  (bind _returnvalue (Transformation|GetActorForwardVector))
  (bind _returnvalue_2 (Transformation|GetActorForwardVector))
  (bind _returnvalue_3 (Transformation|GetActorLocation))
  (bind _returnvalue_4 (Transformation|GetActorLocation))
  (bind _charactermovement (Variables|Character|GetCharacterMovement))
  (bind _charactermovement_2 (Variables|Character|GetCharacterMovement))
  (bind _returnvalue_5 (* _returnvalue 5e+02))
  (bind _returnvalue_6 (* _returnvalue_2 ""))
  ;[1 1 1] wall detection
  (if (AI|Components|NavMovement|IsFalling (Variables|Character|GetCharacterMovement))
    (Utilities|FlowControl|Sequence
      (:then_0
        ;;[1 1 1] check if right side of the wall
        (if (not (Variables|Default|GetIsLeftSide))
          ;;[1 1 1] Run on the right side of the wall
          (bind (_outhit _returnvalue_7) (Collision|LineTraceByChannel _returnvalue_4 (+ _returnvalue_4 (* (Transformation|GetActorRightVector) 50)) "TraceTypeQuery1" false 0 "ForDuration"))
          (if _returnvalue_7
            (Variables|Default|SetIsRightSide true)
            (Variables|Default|SetOnRightSide true)
            (if (not (Variables|Default|GetIsJumpingOffWall))
              (Transformation|SetActorRotation (Math|Rotator|MakeRotator 0.0 0.0 (+ (.yaw (Math|Conversions|RotationFromXVector (.Normal (Collision|BreakHitResult _outhit)))) 9e+01)))
              (Variables|/Script/Engine.MovementComponent|SetVelocity _charactermovement (Math|Vector|MakeVector (.x _returnvalue_5) (.y _returnvalue_5) 0.0))
              (Variables|/Script/Engine.CharacterMovementComponent|SetGravityScale _charactermovement 0.0)
              (Class|MovementComponent|SetPlaneConstraintNormal _charactermovement "0, 0, 0"))
            (else
              (Variables|Default|SetIsRightSide false)
              (CallFunction|OffWall)))))
      (:then_1
        ;;[1 1 1] check if Left side of the wall
        (if (Variables|Default|GetIsRightSide)
          ;;[1 1 1] Run on the Left side of the wall
          (bind (_outhit_2 _returnvalue_8) (Collision|LineTraceByChannel _returnvalue_3 (+ _returnvalue_3 (* (Transformation|GetActorRightVector) -50)) "TraceTypeQuery1" false 0 "ForDuration"))
          (if _returnvalue_8
            (Variables|Default|SetIsLeftSide true)
            (Variables|Default|SetOnRightSide false)
            (if (not (Variables|Default|GetIsJumpingOffWall))
              (Transformation|SetActorRotation (Math|Rotator|MakeRotator 0.0 0.0 (+ (.yaw (Math|Conversions|RotationFromXVector (.Normal (Collision|BreakHitResult _outhit_2)))) -9e+01)))
              (Variables|/Script/Engine.MovementComponent|SetVelocity _charactermovement_2 (Math|Vector|MakeVector (.x _returnvalue_6) (.y _returnvalue_6) 0.0))
              (Variables|/Script/Engine.CharacterMovementComponent|SetGravityScale _charactermovement_2 0.0)
              (Class|MovementComponent|SetPlaneConstraintNormal _charactermovement_2 "0, 0, 0"))
            (else
              (Variables|Default|SetIsLeftSide false)
              (CallFunction|OffWall))))))))

(fn ConstructionScript)